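; MapGround_BP is a ground segment for an endless-runner style level, exposing an end-arrow transform.
; On construction it adds two low and two high wall child actors at random picks from three arrow points, so walls can share a spot.
; Overlapping Box asks the game mode to spawn more map, then destroys the segment after a delay.
; Overlapping ScoreBox adds multiplied points and raises the player's stored walk speed up to a cap.
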(event `self.Box.OnComponentBeginOverlap`
  (params (OverlappedComponent :type "PrimitiveComponent Object Reference") (OtherActor :type "Actor Object Reference") (OtherComp :type "PrimitiveComponent Object Reference") (OtherBodyIndex :type Integer) (bFromSweep :type Boolean) (SweepResult :type "HitResult Structure (by ref)"))
  (bind _asbp_third_person_game_mode (cast `/Game/ThirdPerson/Blueprints/BP_ThirdPersonGameMode` (`GameplayStatics.GetGameMode`)))
  (`/Game/ThirdPerson/Blueprints/BP_ThirdPersonGameMode.SpawnMap` _asbp_third_person_game_mode)
  (`KismetSystemLibrary.Delay` 3.0)
  (`self.K2_DestroyActor`))

(event `self.ScoreBox.OnComponentBeginOverlap`
  (params (OverlappedComponent :type "PrimitiveComponent Object Reference") (OtherActor :type "Actor Object Reference") (OtherComp :type "PrimitiveComponent Object Reference") (OtherBodyIndex :type Integer) (bFromSweep :type Boolean) (SweepResult :type "HitResult Structure (by ref)"))
  (`self.ScorePoints`)
  (bind _asbp_third_person_character (cast `/Game/ThirdPerson/Blueprints/BP_ThirdPersonCharacter` (`GameplayStatics.GetPlayerCharacter` 0)))
  (bind _charactermovement (`Character.CharacterMovement` _asbp_third_person_character))
  (set `CharacterMovementComponent.MaxWalkSpeed` (`/Game/ThirdPerson/Blueprints/BP_ThirdPersonCharacter.Speed_Char` _asbp_third_person_character) _charactermovement)
  (bind _output_get (set `CharacterMovementComponent.MaxWalkSpeed` (`KismetMathLibrary.FClamp` (+ (`CharacterMovementComponent.MaxWalkSpeed` _charactermovement) 20.0) 0.0 1500.0) _charactermovement))
  (set `/Game/ThirdPerson/Blueprints/BP_ThirdPersonCharacter.Speed_Char` _output_get _asbp_third_person_character))

(fn `GetArrowEnd`
  (returns (Transform :type "Transform Structure"))
  (return (`SceneComponent.K2_GetComponentToWorld` (`self.ArrowEnd`))))

(fn `ScorePoints`
  (bind _asbp_third_person_game_mode (cast `/Game/ThirdPerson/Blueprints/BP_ThirdPersonGameMode` (`GameplayStatics.GetGameMode`)))
  (set `/Game/ThirdPerson/Blueprints/BP_ThirdPersonGameMode.CurrentPoints` (+ (`/Game/ThirdPerson/Blueprints/BP_ThirdPersonGameMode.CurrentPoints` _asbp_third_person_game_mode) (* 1 (`/Game/ThirdPerson/Blueprints/BP_ThirdPersonGameMode.PointMulti` _asbp_third_person_game_mode))) _asbp_third_person_game_mode))

(fn `SetSpawnPoints`
  (set `self.SpawnPoints` (`|MakeArray` (`SceneComponent.GetRelativeTransform` (`self.Arrow_Wall_01`)) (`SceneComponent.GetRelativeTransform` (`self.Arrow_Wall_02`)) (`SceneComponent.GetRelativeTransform` (`self.Arrow_Wall_03`)))))

(fn `SpawnHighWall`
  (bind _spawnpoints (`self.SpawnPoints`))
  (`AddComponent|NODE_AddChildActorComponent-3` :`RelativeTransform` (`|GetArrayItem` _spawnpoints (`KismetMathLibrary.RandomIntegerInRange` 0 (`KismetArrayLibrary.Array_LastIndex` _spawnpoints)))))

(fn `SpawnLowWall`
  (bind _spawnpoints (`self.SpawnPoints`))
  (`AddComponent|NODE_AddChildActorComponent-0` :`RelativeTransform` (`|GetArrayItem` _spawnpoints (`KismetMathLibrary.RandomIntegerInRange` 0 (`KismetArrayLibrary.Array_LastIndex` _spawnpoints)))))

(fn `UserConstructionScript`
  (`self.SetSpawnPoints`)
  (`self.SpawnLowWall`)
  (`self.SpawnLowWall`)
  (`self.SpawnHighWall`)
  (`self.SpawnHighWall`))