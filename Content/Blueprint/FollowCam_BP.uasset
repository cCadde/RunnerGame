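; FollowCam_BP is a follow camera actor that tracks a target along the world X axis or scrolls by itself when it has none.
; SetFollow stores the target and the camera's current offset from it.
; Each Tick adds only the target's X position to that offset, so Y and Z stay constant.
; Without a valid target, it moves along world +X by SpeedCam per frame, unscaled by delta time.
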(event `self.ReceiveBeginPlay`
  (set `self.CamPos` (`self.K2_GetActorLocation`)))

(event `self.ReceiveTick`
  (params (DeltaSeconds :type "Float (single-precision)"))
  (bind _char (`self.Char`))
  (bind _returnvalue_x (`KismetMathLibrary.BreakVector` (`self.K2_GetActorLocation` _char)))
  (`/Engine/EditorBlueprintResources/StandardMacros.IsValid` _char
    (:`Is Valid`
      (`self.K2_SetActorLocation` (+ (`KismetMathLibrary.MakeVector` _returnvalue_x) (`self.CamPos`))))
    (:`Is Not Valid`
      (`self.K2_AddActorWorldOffset` (* (`KismetMathLibrary.GetForwardVector` (struct)) (`self.Speed_Cam`))))))

(fn `SetFollow`
  (params (Actor :type "Actor Object Reference"))
  (set `self.Char` Actor)
  (set `self.CamPos` (- (`self.K2_GetActorLocation`) (`self.K2_GetActorLocation` Actor))))

(fn `UserConstructionScript`)